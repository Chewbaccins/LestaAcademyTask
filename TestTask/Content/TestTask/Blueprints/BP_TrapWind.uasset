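; Wind trap that pushes the third-person character while it stands inside the collision box.
; A looping timer periodically turns the Arrow component by a random 0, 90 or 180 degrees to change the wind direction.
; Overlap events track the character, and Tick applies Force along the arrow to its movement component.
; A motionless character also gets a slight forward movement input before the force is applied.
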(event `self.ReceiveBeginPlay`
  (bind _returnvalue (`KismetSystemLibrary.K2_SetTimerDelegate` (delegate `Change Wind`) 2.0 true))
  (set `self.Time Handler` _returnvalue))

(event `Change Wind`
  (bind _arrow (`self.Arrow`))
  (bind (_relativerotation_roll _relativerotation_pitch _relativerotation_yaw) (`KismetMathLibrary.BreakRotator` (`SceneComponent.RelativeRotation` _arrow)))
  (`SceneComponent.K2_SetRelativeRotation` _arrow (`KismetMathLibrary.MakeRotator` 0.0 0.0 (+ _relativerotation_yaw (* (`KismetMathLibrary.RandomInteger` 3) 90.0))) false false))

(event `self.CollisionBox.OnComponentBeginOverlap`
  (params (OverlappedComponent :type "PrimitiveComponent Object Reference") (OtherActor :type "Actor Object Reference") (OtherComp :type "PrimitiveComponent Object Reference") (OtherBodyIndex :type Integer) (bFromSweep :type Boolean) (SweepResult :type "HitResult Structure (by ref)"))
  (bind _asbp_third_person_character (cast `/Game/ThirdPerson/Blueprints/BP_ThirdPersonCharacter` OtherActor))
  (set `self.Character` _asbp_third_person_character)
  (set `self.HasCharacter` true))

(event `self.ReceiveTick`
  (params (DeltaSeconds :type "Float (single-precision)"))
  (if (`self.HasCharacter`)
    (if (== (`self.GetVelocity` (`self.Character`)) (0.0 0.0 0.0))
      (`Pawn.AddMovementInput` (`self.Character`) (`SceneComponent.GetForwardVector` (`Character.CapsuleComponent` (`self.Character`))) 0.1 false))
    (`CharacterMovementComponent.AddForce` (`Character.CharacterMovement` (`self.Character`)) (* (`SceneComponent.GetForwardVector` (`self.Arrow`)) (`self.Force`)))))

(event `self.CollisionBox.OnComponentEndOverlap`
  (params (OverlappedComponent :type "PrimitiveComponent Object Reference") (OtherActor :type "Actor Object Reference") (OtherComp :type "PrimitiveComponent Object Reference") (OtherBodyIndex :type Integer))
  (cast `/Game/ThirdPerson/Blueprints/BP_ThirdPersonCharacter` OtherActor)
  (set `self.HasCharacter` false)
  (set `self.Character` null))

(fn `UserConstructionScript`)