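; BP_RandomDoor is an actor that randomly makes one of two static mesh box groups, left or right, physical each time play begins.
; On BeginPlay a two-way random roll enables physics simulation on six boxes of the chosen side, while this script leaves the other group untouched.
; The construction script is empty and no other logic runs.
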(event `self.ReceiveBeginPlay`
  (switch `int` (`KismetMathLibrary.RandomInteger` 2)
    (:`0`
      (`PrimitiveComponent.SetSimulatePhysics` (`self.SM_Box_Left`) true)
      (`PrimitiveComponent.SetSimulatePhysics` (`self.SM_Box11`) true)
      (`PrimitiveComponent.SetSimulatePhysics` (`self.SM_Box12`) true)
      (`PrimitiveComponent.SetSimulatePhysics` (`self.SM_Box5`) true)
      (`PrimitiveComponent.SetSimulatePhysics` (`self.SM_Box2`) true)
      (`PrimitiveComponent.SetSimulatePhysics` (`self.SM_Box8`) true))
    (:`1`
      (`PrimitiveComponent.SetSimulatePhysics` (`self.SM_Box_Right`) true)
      (`PrimitiveComponent.SetSimulatePhysics` (`self.SM_Box9`) true)
      (`PrimitiveComponent.SetSimulatePhysics` (`self.SM_Box10`) true)
      (`PrimitiveComponent.SetSimulatePhysics` (`self.SM_Box6`) true)
      (`PrimitiveComponent.SetSimulatePhysics` (`self.SM_Box3`) true)
      (`PrimitiveComponent.SetSimulatePhysics` (`self.SM_Box7`) true))))

(fn `UserConstructionScript`)