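; BP_EndGoal is the finish trigger that ends the game when BP_ThirdPersonCharacter overlaps its Box.
; It ragdolls the character's mesh, deactivates its root component, clears its IsActive flag and plays a finish sound.
; It then shows the W_GameCompletion widget with UI-only input and a visible cursor.
; BP_ThirdPersonGameMode supplies the HUD to remove and the time text shown on the completion screen.
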(event `self.Box.OnComponentBeginOverlap`
  (params (OverlappedComponent :type "PrimitiveComponent Object Reference") (OtherActor :type "Actor Object Reference") (OtherComp :type "PrimitiveComponent Object Reference") (OtherBodyIndex :type Integer) (bFromSweep :type Boolean) (SweepResult :type "HitResult Structure (by ref)"))
  (bind _returnvalue (`GameplayStatics.GetPlayerController` 0))
  (bind _asbp_third_person_character (cast `/Game/ThirdPerson/Blueprints/BP_ThirdPersonCharacter` OtherActor))
  (`PrimitiveComponent.SetSimulatePhysics` (`Character.Mesh` _asbp_third_person_character) true)
  (`ActorComponent.SetActive` (`Actor.RootComponent` _asbp_third_person_character) false false)
  (set `/Game/ThirdPerson/Blueprints/BP_ThirdPersonCharacter.IsActive` false _asbp_third_person_character)
  (`GameplayStatics.PlaySound2D` "/Game/TestTask/Music/FinishCue.FinishCue" 1.0 1.0 0.0 null null)
  ;[1 1 1] Handle UI
  (bind _returnvalue_2 (`|CreateWidget` "/Game/TestTask/Widgets/W_GameCompletion.W_GameCompletion_C" _returnvalue))
  (`UserWidget.AddToViewport` _returnvalue_2 0)
  (`WidgetBlueprintLibrary.SetInputMode_UIOnlyEx` _returnvalue _returnvalue_2 "DoNotLock" true)
  (set `PlayerController.bShowMouseCursor` true _returnvalue)
  (bind _asbp_third_person_game_mode (cast `/Game/ThirdPerson/Blueprints/BP_ThirdPersonGameMode` (`GameplayStatics.GetGameMode`)))
  (`Widget.RemoveFromParent` (`/Game/ThirdPerson/Blueprints/BP_ThirdPersonGameMode.W_HUD_ref` _asbp_third_person_game_mode))
  (`/Game/TestTask/Widgets/W_GameCompletion.UpdateTime` _returnvalue_2 (`/Game/ThirdPerson/Blueprints/BP_ThirdPersonGameMode.TimeToText` _asbp_third_person_game_mode)))

(fn `UserConstructionScript`)