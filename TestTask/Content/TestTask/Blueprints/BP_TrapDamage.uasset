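; Floor trap actor that damages the third-person character after a one-second warning, then cools down for five seconds before re-arming.
; StepBox overlap starts a fast looping timer that retriggers the trap while enabled; leaving CollisionBox clears it.
; CollisionBox tracks the player, so damage only lands if they remain inside when the warning ends.
; A dynamic material instance created at construction shows each phase by color, with a click sound on warning.
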(event `self.StepBox.OnComponentBeginOverlap`
  (params (OverlappedComponent :type "PrimitiveComponent Object Reference") (OtherActor :type "Actor Object Reference") (OtherComp :type "PrimitiveComponent Object Reference") (OtherBodyIndex :type Integer) (bFromSweep :type Boolean) (SweepResult :type "HitResult Structure (by ref)"))
  (cast `/Game/ThirdPerson/Blueprints/BP_ThirdPersonCharacter` OtherActor)
  (bind _returnvalue (`KismetSystemLibrary.K2_SetTimerDelegate` (delegate `DamagePlayer`) 0.01 true))
  (set `self.Timer Handler` _returnvalue))

(event `DamagePlayer`
  ;[1 1 1] Is Active?
  (if (`self.TrapEnabled`)
    (set `self.TrapEnabled` false)
    ;[1 1 1] 1 second warning
    (`GameplayStatics.PlaySoundAtLocation` "/Game/TestTask/Music/hard-click_Cue.hard-click_Cue" (`SceneComponent.RelativeLocation` (`self.StepBox`)) (struct) 1.0 1.0 0.0 null null null null)
    (`MaterialInstanceDynamic.SetVectorParameterValue` (`self.Dynamic_MI_ref`) "Color" (struct :`R` 1.0 :`G` 0.162394 :`A` 1.0))
    (`KismetSystemLibrary.Delay` 1.0)
    ;[1 1 1] Deal Damage and 5 sec CD
    (`MaterialInstanceDynamic.SetVectorParameterValue` (`self.Dynamic_MI_ref`) "Color" (struct :`R` 1.0 :`B` 0.017791 :`A` 1.0))
    (`GameplayStatics.ApplyDamage` (`self.OverlappedPlayer`) (`self.Damage`))
    (`KismetSystemLibrary.Delay` 0.1)
    (`MaterialInstanceDynamic.SetVectorParameterValue` (`self.Dynamic_MI_ref`) "Color" (struct :`R` 0.203125 :`G` 0.203125 :`B` 0.203125 :`A` 1.0))
    ;[1 1 1] Reset
    (`KismetSystemLibrary.Delay` 5.0)
    (`MaterialInstanceDynamic.SetVectorParameterValue` (`self.Dynamic_MI_ref`) "Color" (`self.DefaultColor`))
    (set `self.TrapEnabled` true)))

(event `self.CollisionBox.OnComponentBeginOverlap`
  (params (OverlappedComponent :type "PrimitiveComponent Object Reference") (OtherActor :type "Actor Object Reference") (OtherComp :type "PrimitiveComponent Object Reference") (OtherBodyIndex :type Integer) (bFromSweep :type Boolean) (SweepResult :type "HitResult Structure (by ref)"))
  (bind _asbp_third_person_character (cast `/Game/ThirdPerson/Blueprints/BP_ThirdPersonCharacter` OtherActor))
  (set `self.OverlappedPlayer` _asbp_third_person_character))

(event `self.CollisionBox.OnComponentEndOverlap`
  (params (OverlappedComponent :type "PrimitiveComponent Object Reference") (OtherActor :type "Actor Object Reference") (OtherComp :type "PrimitiveComponent Object Reference") (OtherBodyIndex :type Integer))
  (cast `/Game/ThirdPerson/Blueprints/BP_ThirdPersonCharacter` OtherActor)
  (set `self.OverlappedPlayer` null)
  (`KismetSystemLibrary.K2_ClearAndInvalidateTimerHandle` (`self.Timer Handler`)))

(fn `UserConstructionScript`
  (bind _returnvalue (`KismetMaterialLibrary.CreateDynamicMaterialInstance` "/Game/TestTask/Materials/MI_DamageTrap.MI_DamageTrap"))
  (set `self.Dynamic_MI_ref` _returnvalue)
  (`PrimitiveComponent.SetMaterial` (`self.SM_Trap`) 0 (`self.Dynamic_MI_ref`)))